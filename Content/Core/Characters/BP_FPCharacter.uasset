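; First-person player character Blueprint that handles walking, looking and jumping through Enhanced Input.
; On BeginPlay it adds the first-person mapping context to the local player's input subsystem, provided a player controller possesses it.
; Look input drives controller yaw and pitch, while jump input starts and stops the built-in jump.
; Move input follows the control rotation with pitch excluded, so looking up or down does not tilt the movement direction.
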(event `self.ReceiveBeginPlay`
  ;[1 1 1] Setup: BeginPlay
  (bind _asplayer_controller (cast `PlayerController` (`self.GetController`)))
  (bind _returnvalue (pcsubsystem `EnhancedInputLocalPlayerSubsystem` _asplayer_controller))
  (`/Engine/EditorBlueprintResources/StandardMacros.IsValid` _returnvalue
    (:`Is Valid`
      (`EnhancedInputSubsystemInterface.AddMappingContext` _returnvalue "/Game/Core/Characters/Input/FirstPerson/IMC_FirstPerson.IMC_FirstPerson" 0 (struct)))))

(event `EnhancedInput|/Game/Core/Characters/Input/FirstPerson/Actions/IA_Jump_FP`
  (params (ActionValue :type Boolean) (ElapsedSeconds :type "Float (double-precision)") (TriggeredSeconds :type "Float (double-precision)") (InputAction :type "InputAction Object Reference" :default "/Game/Core/Characters/Input/FirstPerson/Actions/IA_Jump_FP.IA_Jump_FP"))
  ;[1 1 1] Input: Jump
  (:`Triggered`
    (`self.Jump`))
  (:`Completed`
    (`self.StopJumping`)))

(event `EnhancedInput|/Game/Core/Characters/Input/FirstPerson/Actions/IA_Look_FP`
  (params (ActionValue :type "Vector2D Structure") (ElapsedSeconds :type "Float (double-precision)") (TriggeredSeconds :type "Float (double-precision)") (InputAction :type "InputAction Object Reference" :default "/Game/Core/Characters/Input/FirstPerson/Actions/IA_Look_FP.IA_Look_FP"))
  ;[1 1 1] Input: CameraLook (Character's Orientation)
  (:`Triggered`
    (`self.AddControllerYawInput` ActionValue_X)
    (`self.AddControllerPitchInput` ActionValue_Y)))

(event `EnhancedInput|/Game/Core/Characters/Input/FirstPerson/Actions/IA_Move_FP`
  (params (ActionValue :type "Vector2D Structure") (ElapsedSeconds :type "Float (double-precision)") (TriggeredSeconds :type "Float (double-precision)") (InputAction :type "InputAction Object Reference" :default "/Game/Core/Characters/Input/FirstPerson/Actions/IA_Move_FP.IA_Move_FP"))
  (bind (_returnvalue_roll _returnvalue_pitch _returnvalue_yaw) (`KismetMathLibrary.BreakRotator` (`self.GetControlRotation`)))
  (bind (_returnvalue_roll_2 _returnvalue_pitch_2 _returnvalue_yaw_2) (`KismetMathLibrary.BreakRotator` (`self.GetControlRotation`)))
  ;[1 1 1] Input: Movement
  (:`Triggered`
    (`self.AddMovementInput` (`KismetMathLibrary.GetRightVector` (`KismetMathLibrary.MakeRotator` _returnvalue_roll 0.0 _returnvalue_yaw)) ActionValue_X)
    (`self.AddMovementInput` (`KismetMathLibrary.GetForwardVector` (`KismetMathLibrary.MakeRotator` 0.0 0.0 _returnvalue_yaw_2)) ActionValue_Y)))

(fn `UserConstructionScript`)